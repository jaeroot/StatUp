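; BP_Circle is a shrinking safe-zone actor that drives damage checks on player characters.
; It stays hidden for a delay after BeginPlay, then appears at a large scale while the Shrink timeline drives both mesh scale and Radius.
; Every Tick, including during the delay, it passes itself to DamageClient on every ThirdPersonCharacter, leaving the damage decision to them.
; Overlap events are empty, and the IsInside logic is disconnected.
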(event OnComponentBeginOverlap(StaticMesh)
  (params (OverlappedComponent :type Primitive%20Component%20Object%20Reference) (OtherActor :type Actor%20Object%20Reference) (OtherComp :type Primitive%20Component%20Object%20Reference) (OtherBodyIndex :type Integer) (bFromSweep :type Boolean) (SweepResult :type Hit%20Result%20Structure%20%28by%20ref%29)))

(event OnComponentEndOverlap(StaticMesh)
  (params (OverlappedComponent :type Primitive%20Component%20Object%20Reference) (OtherActor :type Actor%20Object%20Reference) (OtherComp :type Primitive%20Component%20Object%20Reference) (OtherBodyIndex :type Integer)))

(event Custom|Damage
  (bind _outactors (Actor|GetAllActorsOfClass "/Game/ThirdPersonBP/Blueprints/ThirdPersonCharacter.ThirdPersonCharacter_C"))
  (for _array_element _outactors
    (Default|DamageClient _array_element self)))

(event EventBeginPlay
  (Variables|/Script/Engine.PrimitiveComponent|SetbGenerateOverlapEvents (Variables|컴포넌트|GetStaticMesh) true)
  (Rendering|SetActorHiddenInGame true)
  (Utilities|FlowControl|Delay 27.0)
  (Transformation|SetWorldScale3D (Variables|컴포넌트|GetStaticMesh) "500.000000,500.000000,500.000000")
  (Rendering|SetActorHiddenInGame false)
  (bind _shrink (Timeline|Shrink Play)
    (:Update
      (Transformation|SetWorldScale3D (Variables|컴포넌트|GetStaticMesh) (Math|Conversions|ToVector(Float) _shrink))
      (Variables|Default|SetRadius _shrink))))

(event EventTick
  (params (DeltaSeconds :type Float%20%28single-precision%29))
  (CallFunction|Damage))

(fn ConstructionScript)